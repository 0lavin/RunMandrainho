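; BuildBase is an actor that scrolls continuously along the world X axis in a repeating loop.
; Each Tick offsets the root component by TimetoGo scaled by delta time, so the variable acts as a speed.
; Once it passes a hard-coded X limit, it teleports back to a fixed negative X position, with Y and Z reset to zero.
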(event EventTick
  (params (DeltaSeconds :type Float%20%28single-precision%29))
  (bind _defaultsceneroot (Variables|Default|GetDefaultSceneRoot))
  (Transformation|AddWorldOffset _defaultsceneroot (Math|Vector|MakeVector (* DeltaSeconds (Variables|Default|GetTimetoGo)) 0.0 0.0) false false)
  (if (> (.X (Math|Vector|BreakVector (Transformation|GetWorldLocation _defaultsceneroot))) 6.3e+03)
    (Transformation|SetWorldLocation (Variables|Default|GetDefaultSceneRoot) "-6500.000000, 0, 0" false true)))

(fn ConstructionScript)